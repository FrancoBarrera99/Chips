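; Projectile actor that reports ranged attack hits to its owner through the Gameplay Ability System.
; Its sphere ignores the owner while moving, and the actor destroys itself after a short lifetime.
; On hit, if the owner is a Pawn, it sends an Attack.Range.Hit event with hit target data to that pawn's PlayerState.
; It then spawns a collision emitter at the hit actor's location and destroys itself.
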(event `self.ReceiveBeginPlay`
  (`PrimitiveComponent.IgnoreActorWhenMoving` (`self.Sphere`) (`self.GetOwner`) true)
  (`KismetSystemLibrary.Delay` 1.0)
  (`self.K2_DestroyActor`))

(event `self.ReceiveHit`
  (params (MyComp :type "PrimitiveComponent Object Reference") (Other :type "Actor Object Reference") (OtherComp :type "PrimitiveComponent Object Reference") (bSelfMoved :type Boolean) (HitLocation :type "Vector Structure") (HitNormal :type "Vector Structure") (NormalImpulse :type "Vector Structure") (Hit :type "HitResult Structure (by ref)"))
  (bind _aspawn (cast `Pawn` (`self.GetOwner`)))
  (`AbilitySystemBlueprintLibrary.SendGameplayEventToActor` (`Pawn.PlayerState` _aspawn) (struct :`TagName` "Attack.Range.Hit") (make `GameplayEventData` :`TargetData` (`AbilitySystemBlueprintLibrary.AbilityTargetDataFromHitResult` Hit)))
  (`GameplayStatics.SpawnEmitterAtLocation` (`self.Collision Emitter`) (`self.K2_GetActorLocation` (`.HitActor` (`GameplayStatics.BreakHitResult` Hit))) (struct) (0.6 0.6 0.6))
  (`self.K2_DestroyActor`))

(fn `UserConstructionScript`)